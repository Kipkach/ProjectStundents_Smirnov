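; BP_KillZone is the Arcanoid kill zone that handles lost balls and the player's lives.
; It destroys any actor overlapping it and, when that was the last BP_Ball, decrements its Lifes counter.
; With lives left, it spawns a new ball offset from the platform location stored in the BP_Global game instance.
; At zero lives, it shows W_GameEnd and removes the score and HP widget.
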(event `self.KillZone.OnComponentBeginOverlap`
  (params (OverlappedComponent :type "PrimitiveComponent Object Reference") (OtherActor :type "Actor Object Reference") (OtherComp :type "PrimitiveComponent Object Reference") (OtherBodyIndex :type Integer) (bFromSweep :type Boolean) (SweepResult :type "HitResult Structure (by ref)"))
  (bind _lifes (`self.Lifes`))
  (`self.K2_DestroyActor` OtherActor)
  (cast `/Game/MyLogic/Arcanoid/MapContent/BP_Ball` OtherActor)
  (bind _outactors (`GameplayStatics.GetAllActorsOfClass` "/Game/MyLogic/Arcanoid/MapContent/BP_Ball.BP_Ball_C"))
  (if (== (`KismetArrayLibrary.Array_Length` _outactors) 0)
    (set `self.Lifes` (- _lifes 1))
    (if (== _lifes 0)
      (bind _returnvalue (`|CreateWidget` "/Game/MyLogic/Arcanoid/Interface/W_GameEnd.W_GameEnd_C"))
      (`UserWidget.AddToViewport` _returnvalue 0)
      (bind _foundwidgets (`WidgetBlueprintLibrary.GetAllWidgetsOfClass` "/Game/MyLogic/Arcanoid/Interface/W_Score_and_HP.W_Score_and_HP_C"))
      (`Widget.RemoveFromParent` _foundwidgets)
      (else
        (bind _asbp_global (cast `/Game/MyLogic/Arcanoid/BP_Global` (`GameplayStatics.GetGameInstance`)))
        (bind (_platformlocation_x _platformlocation_y _platformlocation_z) (`KismetMathLibrary.BreakVector` (`/Game/MyLogic/Arcanoid/BP_Global.PlatformLocation` _asbp_global)))
        (`|SpawnActorFromClass` "/Game/MyLogic/Arcanoid/MapContent/BP_Ball.BP_Ball_C" (`KismetMathLibrary.MakeTransform` (`KismetMathLibrary.MakeVector` (- _platformlocation_x 150.0) _platformlocation_y _platformlocation_z)) "Undefined" "OverrideRootScale" null null)))))

(fn `UserConstructionScript`)