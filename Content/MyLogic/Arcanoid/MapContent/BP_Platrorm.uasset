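; Player paddle for the Arcanoid game, moved sideways in fixed Y steps by the MoveRight axis without sweep.
; Each tick it writes its Platform component's location to BP_Global, the game instance.
; Hitting a BP_Bonus destroys it and spawns two balls near the hit point.
; Hitting a BP_Debuf destroys it and, above a minimum scale, narrows the paddle until a retriggerable delay restores a fixed width.
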(event `self.ReceiveTick`
  (params (DeltaSeconds :type "Float (single-precision)"))
  (bind _asbp_global (cast `/Game/MyLogic/Arcanoid/BP_Global` (`GameplayStatics.GetGameInstance`)))
  (set `/Game/MyLogic/Arcanoid/BP_Global.PlatformLocation` (`SceneComponent.K2_GetComponentLocation` (`self.Platform`)) _asbp_global))

(event `InputAxis|MoveRight`
  (params (AxisValue :type "Float (single-precision)"))
  (if (< AxisValue 0.0)
    (`self.K2_AddActorWorldOffset` (0.0 50.0 0.0))))

(event `InputAxis|MoveRight`
  (params (AxisValue :type "Float (single-precision)"))
  (if (> AxisValue 0.0)
    (`self.K2_AddActorWorldOffset` (0.0 -50.0 0.0))))

(event `self.ReceiveHit`
  (params (MyComp :type "PrimitiveComponent Object Reference") (Other :type "Actor Object Reference") (OtherComp :type "PrimitiveComponent Object Reference") (bSelfMoved :type Boolean) (HitLocation :type "Vector Structure") (HitNormal :type "Vector Structure") (NormalImpulse :type "Vector Structure") (Hit :type "HitResult Structure (by ref)"))
  (bind (_returnvalue_x _returnvalue_y _returnvalue_z) (`KismetMathLibrary.BreakVector` (`self.GetActorRelativeScale3D`)))
  (bind _platform (`self.Platform`))
  (cast `/Game/MyLogic/Arcanoid/MapContent/BP_Bonus` Other
    (:`then`
      (`self.K2_DestroyActor` Other)
      (for _ (range 2)
        (`|SpawnActorFromClass` "/Game/MyLogic/Arcanoid/MapContent/BP_Ball.BP_Ball_C" (`KismetMathLibrary.MakeTransform` (`KismetMathLibrary.MakeVector` (+ HitLocation_X (`KismetMathLibrary.RandomFloatInRange` -2.0 2.0)) (+ HitLocation_Y (`KismetMathLibrary.RandomFloatInRange` -2.0 2.0)) HitLocation_Z)) "Undefined" "OverrideRootScale" null null)))
    (:`CastFailed`
      (cast `/Game/MyLogic/Arcanoid/MapContent/BP_Debuf` Other)
      (`self.K2_DestroyActor` Other)
      (if (not (< _returnvalue_x 4.0))
        (`SceneComponent.SetRelativeScale3D` _platform (`KismetMathLibrary.MakeVector` (- _returnvalue_x 3.0) _returnvalue_y _returnvalue_z))
        (`KismetSystemLibrary.RetriggerableDelay` 10.0)
        (`SceneComponent.SetRelativeScale3D` _platform (`KismetMathLibrary.MakeVector` 8.75 _returnvalue_y _returnvalue_z))))))

(fn `UserConstructionScript`)